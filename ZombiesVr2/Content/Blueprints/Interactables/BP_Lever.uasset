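; VR purchase lever that buys and spawns an actor for the player's VRPawn.
; While grabbed, Tick pitches the handle toward the motion controller within clamped limits, re-arming a timer whenever pitch is non-negative.
; When the timer fires, it calls Buy with Price, spawning BoughtActor at ObjectSpawnpoint only once, or printing an insufficient-nanos message.
; Release or that spawn drops the controller, resets the handle and invalidates the timer handle.
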(event `/Game/VRTemplate/Interfaces/BPI_Grab.Grab`
  (params (MotionController :type "MotionControllerComponent Object Reference"))
  (set `self.Motion Controller` MotionController))

(event `/Game/VRTemplate/Interfaces/BPI_Grab.Release`
  (params (MotionController :type "MotionControllerComponent Object Reference"))
  (set `self.Motion Controller` null :!label _label)
  (`SceneComponent.K2_SetRelativeRotation` (`self.Handle`) (`KismetMathLibrary.MakeRotator` 0.0 45.0) false false)
  (`KismetSystemLibrary.K2_InvalidateTimerHandle` (stale `self.ReceiveTick` _returnvalue)))

(event `self.ReceiveTick`
  (params (DeltaSeconds :type "Float (single-precision)"))
  (bind (_relativerotation_roll _relativerotation_pitch) (`KismetMathLibrary.BreakRotator` (`SceneComponent.RelativeRotation` (`self.Handle`))))
  (bind _motion_controller (`self.Motion Controller`)
    (:`then`
      (`|ExecutionSequence`
        (:`then_0`
          (`self.NewFunction` _motion_controller))
        (:`then_1`
          (if (>= _relativerotation_pitch 0.0)
            (bind _returnvalue (`KismetSystemLibrary.K2_SetTimerDelegate` (delegate `TimerForAction`) (`self.Time`)))))))
    (:`else`)))

(event `TimerForAction`
  (bind _canbuy (`/Game/VRTemplate/Blueprints/VRPawn.Buy` (stale `self.ReceiveBeginPlay` _asvrpawn) (`self.Price`)))
  (if _canbuy
    (`/Engine/EditorBlueprintResources/StandardMacros.DoOnce` false
      (:`Completed`
        (`|SpawnActorFromClass` (`self.BoughtActor`) (`self.GetTransform` (`self.ObjectSpawnpoint`)) "Undefined" "MultiplyWithRoot" null null)
        (goto _label)))
    (else
      (`KismetSystemLibrary.PrintString` "Dont have enough nanos"))))

(event `self.ReceiveBeginPlay`
  (bind _asvrpawn (cast `/Game/VRTemplate/Blueprints/VRPawn` (`GameplayStatics.GetPlayerPawn` 0))))

(fn `NewFunction`
  (params (MotioonController :type "SceneComponent Object Reference"))
  (bind _handle (`self.Handle`))
  (bind (_returnvalue_location _returnvalue_rotation _returnvalue_scale) (`KismetMathLibrary.BreakTransform` (`SceneComponent.K2_GetComponentToWorld` (`self.Handle`))))
  (bind (_relativerotation_roll _relativerotation_pitch) (`KismetMathLibrary.BreakRotator` (`SceneComponent.RelativeRotation` _handle)))
  (bind _returnvalue_location_2 (`KismetMathLibrary.BreakTransform` (`KismetMathLibrary.MakeRelativeTransform` (`SceneComponent.K2_GetComponentToWorld` MotioonController) (`KismetMathLibrary.MakeTransform` _returnvalue_location (`KismetMathLibrary.ComposeRotators` _returnvalue_rotation (struct :`Pitch` 90.0)) _returnvalue_scale))))
  (bind (_returnvalue_roll _returnvalue_pitch) (`KismetMathLibrary.BreakRotator` (`KismetMathLibrary.FindLookAtRotation` (`KismetMathLibrary.MakeVector` 0.0) _returnvalue_location_2)))
  (`SceneComponent.K2_SetRelativeRotation` _handle (`KismetMathLibrary.MakeRotator` 0.0 (`KismetMathLibrary.FClamp` (+ _relativerotation_pitch _returnvalue_pitch) -45.0 45.0)) false false)
  (return))

(fn `UserConstructionScript`)